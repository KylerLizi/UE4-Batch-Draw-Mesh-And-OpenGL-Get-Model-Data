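; Actor Blueprint that builds a procedural mesh from vertex and triangle DataTables and converts it to a static mesh at play start.
; GetData reads each row of VerticeData into positions and each row of TrianglesData into three indices.
; The construction script feeds those arrays into a mesh section and applies HueShift_Mat.
; BeginPlay passes the procedural mesh and MeshName to ProceduralMeshConvertToStaticMesh.
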(event EventBeginPlay
  (Class|PMConvertSM|ProceduralMeshConverttoStaticMesh (Variables|Default|GetProceduralMesh) (Variables|Default|GetMeshName)))

(event EventTick
  (params (DeltaSeconds :type Float%20%28single-precision%29)))

(fn ConstructionScript
  (bind _proceduralmesh (Variables|Default|GetProceduralMesh))
  (bind (_vertices _triangles) (CallFunction|GetData))
  (Class|ProceduralMeshComponent|CreateMeshSectionLinearColor _proceduralmesh 0 _vertices _triangles 0 0 0 0 0 0 0 false)
  (Rendering|Material|SetMaterial _proceduralmesh 0 "/Engine/Functions/Engine_MaterialFunctions02/ExampleContent/HueShift_Mat.HueShift_Mat"))

(fn GetData
  (bind _outrownames (DataTable|GetDataTableRowNames (Variables|Default|GetVerticeData)))
  (for _array_element _outrownames
    (bind _returnvalue (Utilities|GetDataTableRow (Variables|Default|GetVerticeData) _array_element)
      (:then
        (Utilities|Array|Add (Variables|Default|GetVertices) (Math|Vector|MakeVector (.Vertice_X (Utilities|Struct|BreakS_Vertice _returnvalue)) (.Vertice_Y (Utilities|Struct|BreakS_Vertice _returnvalue)) (.Vertice_Z (Utilities|Struct|BreakS_Vertice _returnvalue)))))))
  (bind _outrownames_2 (DataTable|GetDataTableRowNames (Variables|Default|GetTrianglesData)))
  (for _array_element_2 _outrownames_2
    (bind _returnvalue_2 (Utilities|GetDataTableRow (Variables|Default|GetTrianglesData) _array_element_2)
      (:then
        (Utilities|Array|Add (Variables|Default|GetTriangles) (.Vertice1 (Utilities|Struct|BreakS_Triangle _returnvalue_2)))
        (Utilities|Array|Add (Variables|Default|GetTriangles) (.Vertice2 (Utilities|Struct|BreakS_Triangle _returnvalue_2)))
        (Utilities|Array|Add (Variables|Default|GetTriangles) (.Vertice3 (Utilities|Struct|BreakS_Triangle _returnvalue_2))))))
  (return (Variables|Default|GetVertices) (Variables|Default|GetTriangles)))